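; BP_Station is a station marker actor that shows demand status as a tinted 3D icon, with an optional cube visualizing a data value.
; The construction script creates a dynamic icon material tinted by Status and, when DataCube is enabled, shows GraphCube with Z scale set from DebugData.
; Each tick, the whole actor rotates to face the player camera.
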(event `UpdateIconColor`
  (`MaterialInstanceDynamic.SetVectorParameterValue` (`self.MID`) "Color Tint" (select `/Game/Blueprints/Data/E_StationStatus` (`self.Status`) :`NewEnumerator0` (make `LinearColor` 1.0 1.0 1.0) :`NewEnumerator1` (make `LinearColor` 0.5 0.5) :`NewEnumerator2` (make `LinearColor` 0.67))))

(event `UpdateGraphCube`
  (`SceneComponent.SetRelativeScale3D` (`self.GraphCube`) (`KismetMathLibrary.MakeVector` 10.0 10.0 (`self.DebugData`))))

(event `self.ReceiveTick`
  (params (DeltaSeconds :type "Float (single-precision)"))
  (`self.K2_SetActorRotation` (`KismetMathLibrary.FindLookAtRotation` (`self.K2_GetActorLocation`) (`PlayerCameraManager.GetCameraLocation` (`GameplayStatics.GetPlayerCameraManager` 0))) true))

(fn `UserConstructionScript`
  (locals (NewLocalVar :type "MaterialInstanceDynamic Object Reference"))
  (`|ExecutionSequence`
    (:`then_0`
      (if (`self.DataCube`)
        (`SceneComponent.SetVisibility` (`self.GraphCube`) (`self.DataCube`) false)
        (`self.UpdateGraphCube`)))
    (:`then_1`
      (bind _returnvalue (`KismetMaterialLibrary.CreateDynamicMaterialInstance` "/Game/Materials/UI/M_Icons_T.M_Icons_T" "MID_Icon"))
      (bind _output_get (set `self.MID` _returnvalue))
      (`PrimitiveComponent.SetMaterial` (`self.Icon3D`) 0 _output_get)
      (`self.UpdateIconColor`))))